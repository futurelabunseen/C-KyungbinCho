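; Game mode for a two-team match that assigns player starts, spawns heroes and reports the server to a gRPC matchmaker.
; On login, each player gets a free BP_PlayerStart on the less-populated team; logout frees it.
; SpawnPlayer possesses the start's hero class, using the start's SpawnTransform actor once the match begins, when everyone respawns.
; Matchmaker update and removal events build the address from the command-line fqdn and server port.
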(event `self.GRPC_UpdateAddressToMatchmaker`
  (bind _returnvalue (`self.GetNumPlayers`))
  (`CallMatchUpdateToMatchmaker.UpdateToMatchmaker` (make `GrpcMatchUpdateRequest` (`self.Get Server Address`) _returnvalue)))

(event `self.GRPC_RemoveAddressFromMatchmaker`
  (`CallMatchRemoveFromMatchmaker.RemoveFromMatchmaker` (make `GrpcMatchRemoveRequest` (`self.Get Server Address`))))

(event `self.ReceiveBeginPlay`
  (bind _outactors (`GameplayStatics.GetAllActorsOfClass` "/Game/Maps/BP_PlayerStart.BP_PlayerStart_C"))
  (set `self.PlayerStart Array` _outactors))

(event `self.K2_PostLogin`
  (params (NewPlayer :type "PlayerController Object Reference"))
  (bind (_asbp_player_state _bsuccess) (cast `/Game/Characters/BP_PlayerState` (`Controller.PlayerState` NewPlayer) :!pure true))
  (if _bsuccess
    (bind _new_player_start (`self.Find New Player Start`))
    (bind _output_get (set `/Game/Characters/BP_PlayerState.Player Start` _new_player_start _asbp_player_state))
    (`self.Spawn Player` NewPlayer)
    (set `/Game/Maps/BP_PlayerStart.Is Player Set` true _output_get)
    (if (`|EnumEquality` (`/Game/Maps/BP_PlayerStart.Player Team` _output_get) "TeamA")
      (set `self.Num Team A Players` (+ (`self.Num Team A Players`) 1))
      (else
        (set `self.Num Team B Players` (+ (`self.Num Team B Players`) 1))))))

(event `self.K2_OnLogout`
  (params (ExitingController :type "Controller Object Reference"))
  (bind (_asbp_player_state _bsuccess) (cast `/Game/Characters/BP_PlayerState` (`Controller.PlayerState` ExitingController) :!pure true))
  (bind _player_start (`/Game/Characters/BP_PlayerState.Player Start` _asbp_player_state))
  (if _bsuccess
    (`/Engine/EditorBlueprintResources/StandardMacros.IsValid` _player_start
      (:`Is Valid`
        (set `/Game/Maps/BP_PlayerStart.Is Player Set` false _player_start)
        (if (`|EnumEquality` (`/Game/Maps/BP_PlayerStart.Player Team` _player_start) "TeamA")
          (set `self.Num Team A Players` (- (`self.Num Team A Players`) 1))
          (else
            (set `self.Num Team B Players` (- (`self.Num Team B Players`) 1))))))))

(event `self.K2_OnSetMatchState`
  (params (NewState :type Name))
  (if (== NewState "InProgress")
    (for _array_element (`GameStateBase.PlayerArray` (`GameplayStatics.GetGameState`))
      (`self.Spawn Player` (`PlayerState.GetPlayerController` _array_element)))
    (`KismetSystemLibrary.PrintString` "Game Started" true true (struct :`G` 0.66 :`B` 1.0 :`A` 1.0) 5.0)))

(fn `Find New Player Start`
  (returns (`New Player Start` :type "/Game/Maps/BP_PlayerStart Object Reference"))
  (for _array_element (`self.PlayerStart Array`)
    (if (and (not (`/Game/Maps/BP_PlayerStart.Is Player Set` _array_element)) (`|EnumEquality` (`/Game/Maps/BP_PlayerStart.Player Team` _array_element) (select `bool` (> (`self.Num Team A Players`) (`self.Num Team B Players`)) :`false` (enumliteral `EGxPlayerTeam` "TeamA") :`true` (enumliteral `EGxPlayerTeam` "TeamB"))))
      (return _array_element)))
  (return null))

(fn `Get Server Address`
  (returns (`Return Value` :type String))
  (bind _returnvalue (`KismetSystemLibrary.GetCommandLine`))
  (bind (_outtokens _outswitches _outparams) (`KismetSystemLibrary.ParseCommandLine` _returnvalue))
  (return (`KismetStringLibrary.Concat_StrStr` (`BlueprintMapLibrary.Map_Find` _outparams "fqdn") ":" (`KismetStringLibrary.Conv_IntToString` (`GxStatics.GetServerPort`)))))

(fn `Spawn Player`
  (params (`Player Controller` :type "PlayerController Object Reference"))
  (bind _returnvalue (`Controller.K2_GetPawn` `Player Controller`))
  (bind (_asbp_player_state _bsuccess) (cast `/Game/Characters/BP_PlayerState` (`Controller.PlayerState` `Player Controller`) :!pure true))
  (bind _player_start (`/Game/Characters/BP_PlayerState.Player Start` _asbp_player_state))
  (bind _returnvalue_2 (`self.GetTransform` (select `bool` (`self.HasMatchStarted`) :`false` _player_start :`true` (`/Game/Maps/BP_PlayerStart.Spawn Transform` _player_start) :!type "PlayerStart Object Reference")))
  (`/Engine/EditorBlueprintResources/StandardMacros.IsValid` _returnvalue
    (:`Is Valid`
      (`self.K2_DestroyActor` _returnvalue))
    (:`Is Not Valid`
      _))
  (if _bsuccess
    (bind _returnvalue_3 (`|SpawnActorFromClass` (`/Game/Maps/BP_PlayerStart.Spawn Hero Class` _player_start) _returnvalue_2 "Undefined" "MultiplyWithRoot" null null))
    (`Controller.Possess` `Player Controller` _returnvalue_3)
    (`/Game/Characters/BP_PlayerController.ClientRPC_SetControlRotation` (cast `/Game/Characters/BP_PlayerController` `Player Controller` :!pure true) (.rotation _returnvalue_2))))

(fn `UserConstructionScript`)