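; BP_Grenade is the HealA hero's biotic grenade, which detonates when its sphere component hits something and then destroys itself.
; On impact it prints the hit point and runs a debug-drawn, pawn-only sphere trace there.
; Each trace hit fires a BioticGrenade gameplay event, but the target actor is wired from the disabled BP_Hero overlap loop, not the trace result.
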(event `self.Sphere.OnComponentHit`
  (params (HitComponent :type "PrimitiveComponent Object Reference") (OtherActor :type "Actor Object Reference") (OtherComp :type "PrimitiveComponent Object Reference") (NormalImpulse :type "Vector Structure") (Hit :type "HitResult Structure (by ref)"))
  (bind (_bblockinghit _binitialoverlap _time _distance _location _impactpoint) (`GameplayStatics.BreakHitResult` Hit))
  (`KismetSystemLibrary.PrintString` (`KismetStringLibrary.Conv_VectorToString` _impactpoint))
  (if false
    (bind _outactors (`KismetSystemLibrary.SphereOverlapActors` _impactpoint 250.0 (`|MakeArray` "ObjectTypeQuery3" :!type "EObjectTypeQuery Enum") "/Game/Characters/BP_Hero.BP_Hero_C"))
    (for _array_element _outactors
      (`AbilitySystemBlueprintLibrary.SendGameplayEventToActor` _array_element (struct :`TagName` "SetByCaller.BioticGrenade") (make `GameplayEventData` (struct :`TagName` "SetByCaller.BioticGrenade")) :!label _label))
    (else
      (bind _outhits (`KismetSystemLibrary.SphereTraceMultiByProfile` :`Start` _impactpoint :`End` _impactpoint :`Radius` 250.0 :`ProfileName` "OverlapOnlyPawn" :`DrawDebugType` "ForDuration"))
      (for _array_element_2 _outhits
        (goto _label))))
  (`self.K2_DestroyActor`))

(fn `UserConstructionScript`)