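; Player controller that marks the BP_Hero nearest the player's line of sight by showing its TargetedComponent.
; BeginPlay caches every other hero; Tick hides all their markers, then sphere-traces from the view point along its forward vector using the SwiftStrike profile.
; Hit heroes are ranked by squared offset projected onto the view-facing plane, so the one closest to the view axis wins regardless of depth.
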(event `self.ReceiveBeginPlay`
  (bind (_asbp_hero _bsuccess) (cast `/Game/Characters/BP_Hero` (`self.K2_GetPawn`) :!pure true))
  (bind _outactors (`GameplayStatics.GetAllActorsOfClass` "/Game/Characters/BP_Hero.BP_Hero_C"))
  (bind _output_get (set `self.HeroActors` _outactors))
  (if _bsuccess
    (`KismetArrayLibrary.Array_RemoveItem` _output_get _asbp_hero)))

(event `self.ReceiveTick`
  (params (DeltaSeconds :type "Float (single-precision)"))
  (bind _nearesthero (`self.NearestHero`))
  (for _array_element (`self.HeroActors`)
    (`SceneComponent.SetVisibility` (`/Game/Characters/BP_Hero.TargetedComponent` _array_element) false false))
  (set `self.MinDistanceSquared` 99999999.0)
  (set `self.NearestHero` null)
  (bind _return_value (`self.Get Sphere Trace Results`))
  (for _array_element_2 _return_value
    (bind (_bblockinghit _binitialoverlap _time _distance _location _impactpoint _normal _impactnormal _physmat _hitactor) (`GameplayStatics.BreakHitResult` _array_element_2))
    (bind _return_value_2 (`self.Get Projected Distance Squared 2D` _hitactor))
    (bind (_asbp_hero _bsuccess) (cast `/Game/Characters/BP_Hero` _hitactor :!pure true))
    (if (and (< _return_value_2 (`self.MinDistanceSquared`)) _bsuccess)
      (set `self.MinDistanceSquared` _return_value_2)
      (set `self.NearestHero` _asbp_hero)))
  (`/Engine/EditorBlueprintResources/StandardMacros.IsValid` _nearesthero
    (:`Is Valid`
      (`SceneComponent.SetVisibility` (`/Game/Characters/BP_Hero.TargetedComponent` _nearesthero) true false))))

(fn `Get Projected Distance Squared 2D`
  (params (InActor :type "Actor Object Reference"))
  (returns (`Return Value` :type "Float (double-precision)"))
  (bind (_location _rotation) (`self.GetPlayerViewPoint`))
  (return (`KismetMathLibrary.VSizeSquared` (`KismetMathLibrary.ProjectVectorOnToPlane` (- (`self.K2_GetActorLocation` InActor) _location) (`KismetMathLibrary.GetForwardVector` _rotation)))))

(fn `Get Sphere Trace Results`
  (returns (`Return Value` :type "Array of HitResult Structure"))
  (bind (_location _rotation) (`self.GetPlayerViewPoint`))
  (bind _outhits (`KismetSystemLibrary.SphereTraceMultiByProfile` _location (+ _location (* (`KismetMathLibrary.GetForwardVector` _rotation) (`self.TraceDistance`))) (`self.TraceRadius`) "SwiftStrike" false (`|MakeArray` (`self.K2_GetPawn`) :!type "Actor Object Reference") "None" true (struct :`R` 1.0 :`A` 1.0) (struct :`G` 1.0 :`A` 1.0) 0.1))
  (return _outhits))

(fn `UserConstructionScript`)